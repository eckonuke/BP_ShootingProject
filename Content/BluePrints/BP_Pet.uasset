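; BP_Pet is a pet actor that continuously moves toward the player's BP_Player actor.
; Each Tick it looks up BP_Player with GetActorOfClass and proceeds only if that reference is valid.
; It normalizes the vector to the player, scales it by Speed and DeltaSeconds, and applies the offset through SetActorLocationAndRotation.
; The movement has no stopping distance, and no target rotation is computed.
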(event `self.ReceiveTick`
  (params (DeltaSeconds :type "Float (single-precision)"))
  ;[1 1 1] Vector
  ;;[1 1 1] V-방향
  (bind _returnvalue (`GameplayStatics.GetActorOfClass` "/Game/BluePrints/BP_Player.BP_Player_C"))
  (`/Engine/EditorBlueprintResources/StandardMacros.IsValid` _returnvalue
    (:`Is Valid`
      ;[1 1 1] Comment
      (`self.K2_SetActorLocationAndRotation` (+ (`self.K2_GetActorLocation`) (* (* (`KismetMathLibrary.Normal` (- (`self.K2_GetActorLocation` _returnvalue) (`self.K2_GetActorLocation`))) (`self.speed`)) DeltaSeconds))))))

(fn `UserConstructionScript`)