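; Game mode that tracks the current score and persists the best score between sessions.
; On BeginPlay it creates the main widget on screen and loads the saved best score from a save slot.
; AddScore increases the current score and, when it beats the best, updates it and immediately writes it to disk through a BP_SaveGame object.
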(event `self.ReceiveBeginPlay`
  (bind _returnvalue (`|CreateWidget` "/Game/UI/BP_MainWidget.BP_MainWidget_C"))
  (`UserWidget.AddToViewport` _returnvalue 0)
  (bind _bestscore (`self.loadScoreData`))
  (set `self.bestScore` _bestscore))

(fn `addScore`
  (params (Point :type Integer))
  (bind _output_get (set `self.currentScore` (+ Point (`self.currentScore`))))
  (if (> _output_get (`self.bestScore`))
    (bind _output_get_2 (set `self.bestScore` _output_get))
    (`self.saveScoreData` _output_get_2)))

(fn `loadScoreData`
  (returns (bestScore :type Integer))
  (bind _returnvalue (`GameplayStatics.DoesSaveGameExist` "bestScoreData"))
  (if _returnvalue
    (bind _returnvalue_2 (`GameplayStatics.LoadGameFromSlot` "bestScoreData"))
    (bind _asbp_save_game (cast `/Game/BluePrints/BP_SaveGame` _returnvalue_2))
    (return (`/Game/BluePrints/BP_SaveGame.ScoreData` _asbp_save_game))))

(fn `saveScoreData`
  (params (SaveScore :type Integer))
  (bind _returnvalue (`GameplayStatics.CreateSaveGameObject` "/Game/BluePrints/BP_SaveGame.BP_SaveGame_C"))
  (bind _output_get (set `self.Save Instance` _returnvalue))
  (set `/Game/BluePrints/BP_SaveGame.ScoreData` SaveScore _output_get)
  (`GameplayStatics.SaveGameToSlot` _output_get "bestScoreData"))

(fn `UserConstructionScript`)