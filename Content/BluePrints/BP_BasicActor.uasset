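; BP_BasicActor is a scratch actor demonstrating basic Blueprint arithmetic, branching and looping.
; On BeginPlay, a For Loop adds the integers 1 to 10 into Sum and prints the result.
; Helper functions add, multiply, take an absolute difference and safely divide two numbers.
; Their calls, along with sign, single-digit and odd/even checks printed in Korean, sit in unconnected chains that never run.
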(event `self.ReceiveBeginPlay`
  ;[1 1 1] For Loop
  (for _index (range 1 11)
    (bind _output_get (set `self.sum` (+ _index (stale _output_get)))))
  (`KismetSystemLibrary.PrintString` (`KismetStringLibrary.Conv_IntToString` _output_get)))

(event `self.ReceiveTick`
  (params (DeltaSeconds :type "Float (single-precision)")))

(event `self.ReceiveActorBeginOverlap`
  (params (OtherActor :type "Actor Object Reference")))

(fn `AddNum`
  (params (num1 :type Integer) (num2 :type Integer))
  (returns (result :type Integer))
  (return (+ num1 num2)))

(fn `DivNum`
  (params (num1 :type Integer) (num2 :type Integer))
  (returns (result :type "Float (double-precision)"))
  (return (`KismetMathLibrary.SafeDivide` (`KismetMathLibrary.Conv_IntToDouble` num1) (`KismetMathLibrary.Conv_IntToDouble` num2))))

(fn `MultiNum`
  (params (num1 :type Integer) (num2 :type Integer))
  (returns (result :type Integer))
  (return (* num1 num2)))

(fn `SubNum`
  (params (num1 :type Integer) (num2 :type Integer))
  (returns (result :type Integer))
  (return (`KismetMathLibrary.Abs_Int` (- num1 num2))))

(fn `UserConstructionScript`)